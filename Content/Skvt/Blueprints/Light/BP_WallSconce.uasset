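; BP_WallSconce is a wall sconce light whose look is driven by its own variables.
; The construction script calls InitLight, which applies brightness, color, inner and outer cone angles, and on/off visibility to the SconceLight component.
; BeginPlay is empty, so the file has no runtime logic for switching or changing the light.
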(event EventBeginPlay)

(fn ConstructionScript
  (CallFunction|InitLight))

(fn InitLight
  (Rendering|Components|Light|SetIntensity (Variables|Default|GetSconceLight) (Variables|Light|GetBrightness))
  (Rendering|Components|Light|SetLightColor (Variables|Default|GetSconceLight) (Variables|Light|GetColor) true)
  (Rendering|Lighting|SetInnerConeAngle (Variables|Default|GetSconceLight) (Variables|Light|GetInner%20Cone%20Angle))
  (Rendering|Lighting|SetOuterConeAngle (Variables|Default|GetSconceLight) (Variables|Light|GetOuter%20Cone%20Angle))
  (Rendering|SetVisibility (Variables|Default|GetSconceLight) (Variables|Light|GetIsOn) false))